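; First-person rifle that attaches to its owning BP_LearningCharacter on BeginPlay and flags it as having a gun.
; OnFire checks reloading and magazine ammo, then spawns a projectile from the muzzle socket along camera rotation with sound and a montage.
; OnReloadAmmo fills the magazine from passed-in reserve ammo and returns the leftover.
; OnAim moves the weapon mesh between camera and arms, toggling the display mesh's visibility.
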(event EventBeginPlay
  ;[1 1 1] Attach Gun to Player
  (|CallParentFunction)
  (bind _asbp_learning_character (Utilities|Casting|CastToBP_LearningCharacter (Components|GetOwner)))
  (bind _output_get (Variables|Default|SetAs%20BP%20Learning%20Character _asbp_learning_character))
  (Actor|SetOwner _asbp_learning_character)
  (Transformation|AttachComponentToComponent (Variables|/Game/AnimStarterPack/UE4_Mannequin/Mesh/BP_LearningCharacter.BP_LearningCharacter_C|Get1P _output_get) "Riffle" "SnapToTarget" "SnapToTarget" "SnapToTarget" true)
  (Utilities|IsValid (Variables|Default|GetAs%20BP%20Learning%20Character)
    (:Is%20Valid
      (Variables|/Game/AnimStarterPack/UE4_Mannequin/Mesh/BP_LearningCharacter.BP_LearningCharacter_C|SetHasGun (Variables|Default|GetAs%20BP%20Learning%20Character) true))))

(fn ConstructionScript)

(fn OnFire
  (if (not (Variables|Default|GetIsReloading))
    (bind _hasammo_ (CallFunction|ConsumeAmmo))
    (if _hasammo_
      (CallFunction|Fire)
      (return true)
      (else
        (return false)))))

(fn Fire
  (bind _returnvalue (Components|GetOwner))
  (bind _returnvalue_2 (Game|GetPlayerCameraManager 0))
  (bind _projectileoffset (Variables|Default|GetProjectileOffset))
  (bind _weapon1p (Variables|Default|GetWeapon1P))
  (bind _returnvalue_3 (Camera|GetCameraRotation _returnvalue_2))
  (bind _returnvalue_4 (Transformation|GetSocketLocation _weapon1p "BulletSpawnPoint"))
  (bind _returnvalue_5 (Math|Vector|RotateVector _projectileoffset _returnvalue_3))
  (bind _returnvalue_6 (+ _returnvalue_4 _returnvalue_5))
  (Game|SpawnActorfromClass "/Game/FirstPerson/Blueprints/BP_FirstPersonProjectile.BP_FirstPersonProjectile_C" (Math|Transform|MakeTransform _returnvalue_6 _returnvalue_3) "Undefined" "MultiplyWithRoot" _returnvalue (.AsPawn (Utilities|Casting|CastToPawn _returnvalue)))
  (Audio|PlaySoundatLocation "/Game/FPWeapon/Audio/FirstPersonTemplateWeaponFire02.FirstPersonTemplateWeaponFire02" _returnvalue_6 "0, 0, 0" 1.0 1.0 0.0 0 0 0 0)
  (Animation|Montage|MontagePlay (Components|SkeletalMesh|GetAnimInstance (Variables|/Game/AnimStarterPack/UE4_Mannequin/Mesh/BP_LearningCharacter.BP_LearningCharacter_C|Get1P (Variables|Default|GetAs%20BP%20Learning%20Character))) "/Game/FirstPersonArms/Animations/FP_Rifle_Shoot_Montage.FP_Rifle_Shoot_Montage" 1.0 "MontageLength" 0.0 true))

(fn ConsumeAmmo
  (if (<= (Variables|Default|GetAmmo) 0)
    (return false)
    (else
      (bind _output_get (Variables|Default|SetAmmo (- (Variables|Default|GetAmmo) 1)))
      (return true))))

(fn CanReload
  (return (< (Variables|Default|GetAmmo) (Variables|Default|GetMax_Ammo))))

(fn OnReloadAmmo
  (params (Ammo_Inv :type Integer))
  (bind _max_ammo (Variables|Default|GetMax_Ammo))
  (LocalVariables|SetCur_Ammo (Variables|Default|GetAmmo))
  (Variables|Default|SetAmmo (Math|Integer|SelectInt (+ Ammo_Inv (LocalVariables|GetCur_Ammo)) _max_ammo (<= (+ Ammo_Inv (LocalVariables|GetCur_Ammo)) _max_ammo)))
  (return (Math|Integer|Max(Integer) (- (+ Ammo_Inv (LocalVariables|GetCur_Ammo)) (Variables|Default|GetAmmo)))))

(fn GetAmmoNum
  (return (Variables|Default|GetAmmo)))

(fn OnAim
  (params (IsTrue :type Boolean))
  (bind _as_bp_learning_character (Variables|Default|GetAs%20BP%20Learning%20Character))
  (bind _weapon1p (Variables|Default|GetWeapon1P))
  (bind _1p (Variables|/Game/AnimStarterPack/UE4_Mannequin/Mesh/BP_LearningCharacter.BP_LearningCharacter_C|Get1P _as_bp_learning_character))
  (bind _output_get (Variables|Default|SetIsAiming IsTrue))
  (if _output_get
    (Transformation|AttachComponentToComponent _weapon1p (Variables|/Game/AnimStarterPack/UE4_Mannequin/Mesh/BP_LearningCharacter.BP_LearningCharacter_C|GetCamera1 _as_bp_learning_character) "GripPoint_Display" "SnapToTarget" "SnapToTarget" "SnapToTarget" true)
    (Transformation|SetRelativeTransform (Variables|Default|GetWeapon1P) (Math|Transform|MakeTransform "0.000000,0.000000,-20.000000" "0.000000,-90.000000,0.000000" "1.000000,1.000000,1.000000") false false)
    (Development|SetHiddeninGame (Variables|Default|GetWeapon1PDisplay) true false)
    (else
      (Transformation|AttachComponentToComponent _weapon1p _1p "GripPoint_Display" "SnapToTarget" "SnapToTarget" "SnapToTarget" true)
      (Transformation|AttachComponentToComponent (Variables|Default|GetWeapon1P) _1p "GripPoint_Display" "SnapToTarget" "SnapToTarget" "SnapToTarget" true)
      (Development|SetHiddeninGame (Variables|Default|GetWeapon1PDisplay) false false))))