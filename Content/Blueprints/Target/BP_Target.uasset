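; BP_Target is a shootable target whose mesh moves between Right and Left markers on a timeline started at BeginPlay.
; Any hit on the mesh spawns a replacement BP_Target around a fixed point, with clamped random Y/Z position, random roll and varied scale.
; Only a BP_FirstPersonProjectile hit then destroys both target and projectile and sends the score to the first BP_ScoreActor found.
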(event OnComponentHit(StaticMesh)
  (params (HitComponent :type Primitive%20Component%20Object%20Reference) (OtherActor :type Actor%20Object%20Reference) (OtherComp :type Primitive%20Component%20Object%20Reference) (NormalImpulse :type Vector :default "0, 0, 0") (Hit :type Hit%20Result%20Structure%20%28by%20ref%29))
  (bind _returnvalue (Math|Random|RandomUnitVector))
  (bind _vector (Variables|Default|GetVector))
  (Utilities|FlowControl|Sequence
    (:then_0
      (Utilities|FlowControl|Sequence
        (:then_0
          (bind _output_get (Variables|Default|SetBiasX 1000)))
        (:then_1
          (bind _output_get_2 (Variables|Default|SetCoeffecient 2000)))
        (:then_2
          (bind _output_get_3 (Variables|Default|SetBiasY 2000)))
        (:then_3
          (bind _output_get_4 (Variables|Default|SetCoeffecient 4000)))
        (:then_4
          (bind _output_get_5 (Variables|Default|SetZ (+ (- (* (.z _returnvalue) _output_get_2) _output_get) (.z _vector)))))
        (:then_5
          (bind _output_get_6 (Variables|Default|SetY (+ (- (* (.y _returnvalue) _output_get_4) _output_get_3) (.y _vector)))))
        (:then_6
          (if (> _output_get_5 1.6e+03)
            (Variables|Default|SetZ 1.6e+03)))
        (:then_7
          (if (< _output_get_5 4e+02)
            (Variables|Default|SetZ 4e+02)))
        (:then_8
          (if (> _output_get_6 3.6e+03)
            (Variables|Default|SetY 3.6e+03)))
        (:then_9
          (if (< _output_get_6 4e+02)
            (Variables|Default|SetY 4e+02)))
        (:then_10
          (bind _output_get_7 (Variables|Default|SetTransform (Math|Vector|MakeVector (.x _vector) (Variables|Default|GetY) (Variables|Default|GetZ))))
          (bind _output_get_8 (Variables|Default|SetNewRotation (Math|Transform|MakeTransform _output_get_7 (Math|Rotator|MakeRotator (.roll (Math|Random|RandomRotator true)) 0.0 0.0) (Math|Vector|MakeVector 1.0 (Math|Random|RandomFloatinRange 0.8 1.2) (Math|Random|RandomFloatinRange 0.8 1.2)))))
          (Game|SpawnActorfromClass "BP_Target_C" _output_get_8 "AlwaysSpawn" "MultiplyWithRoot" 0 0))))
    (:then_1
      (Utilities|Casting|CastToBP_FirstPersonProjectile OtherActor)
      (Actor|DestroyActor)
      (Actor|DestroyActor OtherActor)
      (CallFunction|OnUpdateScore))))

(event Custom|OnUpdateScore
  (bind _outactors (Actor|GetAllActorsOfClass "/Game/Blueprints/Target/BP_ScoreActor.BP_ScoreActor_C"))
  (Default|OnScoreUpdate (Utilities|Array|Get(acopy) _outactors) (Variables|Default|GetScore)))

(event EventBeginPlay
  (Variables|Default|SetScore 1)
  (Variables|Default|SetVector "-60.000000,2000.000000,1000.000000")
  (bind _movement (Timeline|Movement Play)
    (:Update
      (Transformation|SetRelativeLocation (Variables|Default|GetStaticMesh) (Math|Vector|Lerp(Vector) (Variables|/Script/Engine.SceneComponent|GetRelativeLocation (Variables|Default|GetRight)) (Variables|/Script/Engine.SceneComponent|GetRelativeLocation (Variables|Default|GetLeft)) _movement) false false))))

(event Collision|EventActorBeginOverlap
  (params (OtherActor :type Actor%20Object%20Reference)))

(event EventTick
  (params (DeltaSeconds :type Float%20%28single-precision%29)))

(fn ConstructionScript)