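; Level manager that handles a set of enemies and tracks kills toward a level target.
; BeginPlay sets the kill goal from the Enemies count, and OnTargetKilled increments the tally, calling TargetFinished once the goal is reached.
; RecordEnemies saves enemy transforms, which SpawnEnemies uses to destroy and respawn BP_NewEnemy actors without resetting the tally.
; ActiveEnemies passes an active flag to every valid enemy.
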(event EventBeginPlay
  (Variables|Default|SetTargetKillingGoal (Utilities|Array|Length (Variables|Default|GetEnemies))))

(event Collision|EventActorBeginOverlap
  (params (OtherActor :type Actor%20Object%20Reference)))

(event EventTick
  (params (DeltaSeconds :type Float%20%28single-precision%29)))

(fn ConstructionScript)

(fn SpawnEnemies
  (for _array_element (Variables|Default|GetEnemies)
    (Utilities|IsValid _array_element
      (:Is%20Valid
        (Actor|DestroyActor _array_element))
      (:Is%20Not%20Valid
        (Development|PrintString "SpawnFalied!!!!!!"))))
  (Utilities|Array|Clear (Variables|Default|GetEnemies))
  (for _array_element_2 (Variables|Default|GetEnemiesTrans)
    (bind _returnvalue (Game|SpawnActorfromClass "/Game/AnimStarterPack/UE4_Mannequin/Mesh/BP_NewEnemy.BP_NewEnemy_C" _array_element_2 "Undefined" "MultiplyWithRoot" 0 0))
    (Utilities|Array|Add (Variables|Default|GetEnemies) _returnvalue)))

(fn RecordEnemies
  (for _array_element (Variables|Default|GetEnemies)
    (Utilities|Array|Add (Variables|Default|GetEnemiesTrans) (Transformation|GetActorTransform _array_element))))

(fn ActiveEnemies
  (params (IsActive :type Boolean))
  (for _array_element (Variables|Default|GetEnemies)
    (Utilities|IsValid _array_element
      (:Is%20Valid
        (Default|ActiveEnemy _array_element IsActive)))))

(fn OnTargetKilled
  (Math|Integer|IncrementInt (Variables|Default|GetTargetKilledNum)
    (:%20%20
      (bind _output_get (Variables|Default|SetTargetKilledNum (Variables|Default|GetTargetKilledNum)))
      (if (>= _output_get (Variables|Default|GetTargetKillingGoal))
        (Default|CallTargetFinished)))))