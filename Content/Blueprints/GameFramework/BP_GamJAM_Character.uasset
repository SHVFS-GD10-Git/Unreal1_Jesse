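; First-person player character for the GamJAM game, handling movement, look, jumping, sprinting and rifle shooting.
; BeginPlay spawns a gun and attaches it to the arms mesh socket; Tick copies control pitch onto the camera.
; Shooting plays a montage and sound, spawns a projectile from the gun's Ammo socket along camera rotation, then notifies the first BP_ScoreActor found.
; Sprint toggles walk speed and a flag.
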(event Input|EnhancedActionEvents|EnhancedInputActionIA_Jump
  (params (ActionValue :type Boolean) (ElapsedSeconds :type Float%20%28double-precision%29) (TriggeredSeconds :type Float%20%28double-precision%29) (InputAction :type Input%20Action%20Object%20Reference :default "/Game/FirstPerson/Input/Actions/IA_Jump.IA_Jump"))
  (:Started
    (Character|Jump)))

(event EventTick
  (params (DeltaSeconds :type Float%20%28single-precision%29))
  (bind _camera (Variables|Default|GetCamera))
  (bind _returnvalue (Transformation|GetWorldRotation _camera))
  (|CallParentFunction DeltaSeconds)
  (Transformation|SetWorldRotation _camera (Math|Rotator|MakeRotator (.roll _returnvalue) (.Pitch (Math|Rotator|BreakRotator (Pawn|GetControlRotation (Game|Player|GetPlayerPawn 0) :!class /Script/Engine.Pawn))) (.yaw _returnvalue)) false false))

(event Collision|EventActorBeginOverlap
  (params (OtherActor :type Actor%20Object%20Reference)))

(event EventBeginPlay
  (bind _returnvalue (Game|SpawnActorfromClass "/Game/Blueprints/weapon/Thisistruegun.Thisistruegun_C" (Math|Transform|MakeTransform "0, 0, 0") "Undefined" "MultiplyWithRoot" self 0))
  (bind _output_get (Variables|Default|SetBP%20Gun _returnvalue))
  (Transformation|AttachComponentToComponent _output_get (Variables|Default|GetMesh1P) "Riffle" "SnapToTarget" "SnapToTarget" "SnapToTarget" true))

(event Input|ActionEvents|InputActionShoot
  (params (Key :type Key%20Structure :default "None"))
  (bind _returnvalue (Game|GetPlayerCameraManager 0))
  (bind _bp_gun (Variables|Default|GetBP%20Gun))
  (bind _projectile_offset (Variables|Default|GetProjectile%20Offset))
  (bind _returnvalue_2 (Camera|GetCameraRotation _returnvalue))
  (bind _weapongun (Variables|/Game/Blueprints/weapon/Thisistruegun.Thisistruegun_C|GetWeaponGun _bp_gun))
  (bind _returnvalue_3 (Math|Vector|RotateVector _projectile_offset _returnvalue_2))
  (bind _returnvalue_4 (Transformation|GetSocketLocation _weapongun "Ammo"))
  (bind _returnvalue_5 (+ _returnvalue_4 _returnvalue_3))
  ;[0.05 0.05 0.05] Projectile Spawn Logic
  (:Pressed
    (Animation|Montage|MontagePlay (Components|SkeletalMesh|GetAnimInstance (Variables|Default|GetMesh1P)) "/Game/FirstPersonArms/Animations/FP_Rifle_Shoot_Montage.FP_Rifle_Shoot_Montage" 1.0 "MontageLength" 0.0 true)
    (Game|SpawnActorfromClass "/Game/FirstPerson/Blueprints/BP_FirstPersonProjectile.BP_FirstPersonProjectile_C" (Math|Transform|MakeTransform _returnvalue_5 _returnvalue_2) "Undefined" "OverrideRootScale" 0 0)
    (Audio|PlaySoundatLocation "/Game/FPWeapon/Audio/FirstPersonTemplateWeaponFire02.FirstPersonTemplateWeaponFire02" _returnvalue_5 "0, 0, 0" 1.0 1.0 0.0 0 0 0 0) ; Play firing sound
    (bind _outactors (Actor|GetAllActorsOfClass "/Game/Blueprints/Target/BP_ScoreActor.BP_ScoreActor_C"))
    (Default|OnShoot (Utilities|Array|Get(acopy) _outactors))))

(event Input|ActionEvents|InputActionSprint
  (params (Key :type Key%20Structure :default "None"))
  (bind _charactermovement (Variables|Character|GetCharacterMovement))
  (:Pressed
    (Variables|/Script/Engine.CharacterMovementComponent|SetMaxWalkSpeed _charactermovement 4e+03)
    (Variables|Default|SetIsSprinting true))
  (:Released
    (Variables|/Script/Engine.CharacterMovementComponent|SetMaxWalkSpeed _charactermovement 6e+02)
    (Variables|Default|SetIsSprinting false)))

(event Input|ActionEvents|InputActionJump
  (params (Key :type Key%20Structure :default "None"))
  (:Pressed
    (Character|Jump)))

(event Input|AxisEvents|InputAxisMoveForward
  (params (AxisValue :type Float%20%28single-precision%29))
  (Pawn|Input|AddMovementInput (Transformation|GetActorForwardVector) AxisValue false))

(event Input|AxisEvents|InputAxisMoveRight
  (params (AxisValue :type Float%20%28single-precision%29))
  (Pawn|Input|AddMovementInput (Transformation|GetActorRightVector) AxisValue false))

(event Input|AxisEvents|InputAxisLookUp
  (params (AxisValue :type Float%20%28single-precision%29))
  (Pawn|Input|AddControllerPitchInput AxisValue))

(event Input|AxisEvents|InputAxisLookAround
  (params (AxisValue :type Float%20%28single-precision%29))
  (Pawn|Input|AddControllerYawInput AxisValue))

(fn ConstructionScript)