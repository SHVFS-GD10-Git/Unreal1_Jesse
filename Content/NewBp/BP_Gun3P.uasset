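; BP_Gun3P is a third-person rifle that attaches to the owning BP_LearningCharacter's 3P mesh at BeginPlay.
; OnFire checks reloading and consumes ammo, then spawns a projectile at the muzzle socket using character rotation, with sound and a fire montage.
; Helper functions report ammo and reload eligibility.
; The reload function clamps to MaxAmmo and returns overflow, but adds zero instead of its AmmoInv input.
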(event EventBeginPlay
  (|CallParentFunction)
  (bind _asbp_learning_character (Utilities|Casting|CastToBP_LearningCharacter (Components|GetOwner)))
  (bind _output_get (Variables|Default|SetAs%20BP%20Learning%20Character _asbp_learning_character))
  (Actor|SetOwner _output_get)
  (Transformation|AttachComponentToComponent (Variables|/Game/AnimStarterPack/UE4_Mannequin/Mesh/BP_LearningCharacter.BP_LearningCharacter_C|Get3P _output_get) "RIfleHandle" "SnapToTarget" "SnapToTarget" "SnapToTarget" true))

(fn ConstructionScript)

(fn OnFire
  (if (not (Variables|Default|GetIsReloading))
    (bind _hasammo_ (CallFunction|ConsumeAmmo))
    (if _hasammo_
      (CallFunction|Fire)
      (return true)
      (else
        (return false)))))

(fn Fire
  (bind _returnvalue (Components|GetOwner))
  (bind _aspawn (Utilities|Casting|CastToPawn _returnvalue))
  (Game|SpawnActorfromClass "/Game/FirstPerson/Blueprints/BP_FirstPersonProjectile.BP_FirstPersonProjectile_C" (Math|Transform|MakeTransform (Transformation|GetSocketLocation (Variables|Default|GetGun3p) "BulletSpawnPoint") (Transformation|GetActorRotation (Variables|Default|GetAs%20BP%20Learning%20Character))) "Undefined" "MultiplyWithRoot" _aspawn _aspawn)
  (Audio|PlaySoundatLocation "/Game/FPWeapon/Audio/FirstPersonTemplateWeaponFire02.FirstPersonTemplateWeaponFire02" (Transformation|GetActorLocation self) "0, 0, 0" 1.0 1.0 0.0 0 0 0 0)
  (Animation|Montage|MontagePlay (Components|SkeletalMesh|GetAnimInstance (Variables|/Game/AnimStarterPack/UE4_Mannequin/Mesh/BP_LearningCharacter.BP_LearningCharacter_C|Get3P (Variables|Default|GetAs%20BP%20Learning%20Character))) "/Game/AnimStarterPack/UE4_Mannequin/Mesh/Montage/Fire_Rifle_Hip_Montage.Fire_Rifle_Hip_Montage" 1.0 "MontageLength" 0.0 true))

(fn ConsumeAmmo
  (if (<= (Variables|Default|GetAmmo) 0)
    (return false)
    (else
      (bind _output_get (Variables|Default|SetAmmo (- (Variables|Default|GetAmmo) 1)))
      (return true))))

(fn CanReload
  (return (< (Variables|Default|GetAmmo) (Variables|Default|GetMaxAmmo))))

(fn OnReloadAmmo
  (params (AmmoInv :type Integer))
  (bind _maxammo (Variables|Default|GetMaxAmmo))
  (Variables|Default|SetCur_Ammo (Variables|Default|GetAmmo))
  (Development|PrintString (Utilities|String|ToString(Integer) 0))
  (Variables|Default|SetAmmo (Math|Integer|SelectInt (+ 0 (Variables|Default|GetCur_Ammo)) _maxammo (<= (+ 0 (Variables|Default|GetCur_Ammo)) _maxammo)))
  (return (Math|Integer|Max(Integer) (- (+ 0 (Variables|Default|GetCur_Ammo)) (Variables|Default|GetAmmo)))))

(fn GetAmmoNum
  (return (Variables|Default|GetAmmo)))